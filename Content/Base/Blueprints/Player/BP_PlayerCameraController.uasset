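; Player camera controller that handles mouse-over highlighting of Equipment actors.
; Tick, throttled by a short Delay, runs HoverEquipment, which casts the actor under the cursor to Equipment and swaps hovered state and highlight, preserving the selected item's highlight.
; Hover clears over non-Equipment actors but persists when the cursor hits no actor.
; Q prints the GameInstance class name for debugging; other debug prints and a line trace are disconnected.
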(event EventBeginPlay
  (|CallParentFunction))

(event EventTick
  (params (DeltaSeconds :type Float%20%28single-precision%29))
  (|CallParentFunction DeltaSeconds)
  (Utilities|FlowControl|Delay 0.02)
  (CallFunction|HoverEquipment))

(event Input|KeyboardEvents|Q
  (params (Key :type Key%20Structure :default "AnyKey"))
  (:Pressed
    (Development|PrintString (Utilities|GetClassDisplayName (Utilities|GetClass (Game|GetGameInstance))))))

(fn ConstructionScript)

(fn HoverEquipment
  (bind _hitresult (Game|Player|GetHitResultUnderCursorbyChannel "TraceTypeQuery3" false))
  (bind (_bblockinghit _binitialoverlap _time _location _impactpoint _normal _impactnormal _physmat _hitactor) (Collision|BreakHitResult _hitresult))
  (if (Utilities|IsValid _hitactor)
    (bind _asequipment (Utilities|Casting|CastToEquipment _hitactor)
      (:then
        (LocalVariables|SetHitEquipment _asequipment)
        (if (!= (LocalVariables|GetHitEquipment) (Class|PlayerCameraController|GetSelectedEquipment))
          (if (!= (LocalVariables|GetHitEquipment) (Class|PlayerCameraController|GetHoveredEquipment))
            (if (and (Utilities|IsValid (Class|PlayerCameraController|GetHoveredEquipment)) (!= (Class|PlayerCameraController|GetSelectedEquipment) (Class|PlayerCameraController|GetHoveredEquipment)))
              (Class|Equipment|SetEquipmentHighlight (Class|PlayerCameraController|GetHoveredEquipment) false))
            (Class|PlayerCameraController|SetHoveredEquipment (LocalVariables|GetHitEquipment))
            (Class|Equipment|SetEquipmentHighlight (LocalVariables|GetHitEquipment) true))
          (elif (and (Utilities|IsValid (Class|PlayerCameraController|GetHoveredEquipment)) (!= (Class|PlayerCameraController|GetSelectedEquipment) (Class|PlayerCameraController|GetHoveredEquipment)))
            (Class|Equipment|SetEquipmentHighlight (Class|PlayerCameraController|GetHoveredEquipment) false)
            (Class|PlayerCameraController|SetHoveredEquipment (LocalVariables|GetHitEquipment)))))
      (:CastFailed
        (if (Utilities|IsValid (Class|PlayerCameraController|GetHoveredEquipment))
          (if (!= (Class|PlayerCameraController|GetSelectedEquipment) (Class|PlayerCameraController|GetHoveredEquipment))
            (Class|Equipment|SetEquipmentHighlight (Class|PlayerCameraController|GetHoveredEquipment) false))
          (Class|PlayerCameraController|SetHoveredEquipment))))))