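; BP_BotGameModeBase is a game mode Blueprint that registers the Bot actors in the level at startup.
; Shortly after BeginPlay, a brief delay precedes a search for all Bot actors, each passed to AddBot.
; A second pass hands every Bot to the first player's PlayerCameraController as a controlled bot, provided the controller cast succeeds.
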(event EventBeginPlay
  (Utilities|FlowControl|Delay 0.2)
  (Utilities|FlowControl|Sequence
    (:then_0
      (bind _outactors (Actor|GetAllActorsOfClass "/Script/BotGame.Bot"))
      (for _array_element _outactors
        (Class|BotGameModeBase|AddBot _array_element)))
    (:then_1
      (bind _outactors_2 (Actor|GetAllActorsOfClass "/Script/BotGame.Bot"))
      (bind _asplayer_camera_controller (Utilities|Casting|CastToPlayerCameraController (Game|GetPlayerController 0)))
      (for _array_element_2 _outactors_2
        (Class|PlayerCameraController|AddControlledBot _asplayer_camera_controller _array_element_2)))))

(fn ConstructionScript)