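; Burnt ground decal actor for the dynamic grass system that grows a scorch mark over the burn duration.
; Construction applies a random yaw and the configured decal material.
; On BeginPlay it picks a randomized per-axis target scale and starts a timeline rate-matched to the burn duration.
; A looping quarter-second timer, rather than timeline updates, lerps actor scale from zero by the timeline alpha and is cleared on finish.
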(event Custom|UpdateBurningGround
  ;[1 1 1] Scale the decal over time, for the burn duration. After this is done, clear the timer.
  (Transformation|SetActorScale3D (Math|Vector|Lerp(Vector) "0, 0, 0" (Variables|Default|GetrandomizedEndGroundScale) (stale EventBeginPlay _alpha))))

(event EventBeginPlay
  (bind _scalerandomizationlevel (Variables|Default|GetscaleRandomizationLevel))
  (bind _scale (Variables|Default|GetScale))
  (bind _returnvalue (- _scale _scalerandomizationlevel))
  (bind _returnvalue_2 (+ _scale _scalerandomizationlevel))
  (bind _returnvalue_3 (Math|Random|RandomFloatinRange _returnvalue _returnvalue_2))
  ;[1 1 1] Calculate randomized end ground scale and set starting (current) scale to 0.
  (Variables|Default|SetrandomizedEndGroundScale (Math|Vector|MakeVector _returnvalue_3 _returnvalue_3 _returnvalue_3))
  (Transformation|SetActorScale3D "0, 0, 0")
  ;[1 1 1] Scale the decal over time, for the burn duration. After this is done, clear the timer.
  (Components|Timeline|SetPlayRate (Variables|Default|GetTimeline_Ground) (/ 1.0 (Variables|Default|GetburnDuration)))
  (Utilities|FlowControl|Sequence
    (:then_0
      (bind _returnvalue_4 (Utilities|Time|SetTimerbyEvent (delegate Custom|UpdateBurningGround) 0.25 true))
      (Variables|Default|Settimer _returnvalue_4))
    (:then_1
      (bind _alpha (Timeline|Timeline_Ground PlayFromStart)
        (:Finished
          (Utilities|Time|ClearandInvalidateTimerbyHandle (Variables|Default|Gettimer)))))))

(fn ConstructionScript
  ;[1 1 1] Add random yaw to the decal and set its material.
  (Transformation|AddActorLocalRotation (Math|Rotator|MakeRotator 0.0 0.0 (Math|Random|RandomFloatinRange -3.6e+02 3.6e+02)) false false)
  (Rendering|Components|Decal|SetDecalMaterial (Variables|Default|GetDecal) (Variables|Default|Getmaterial)))