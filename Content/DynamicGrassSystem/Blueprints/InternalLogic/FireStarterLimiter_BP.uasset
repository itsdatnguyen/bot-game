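; Fire starter limiter actor in the dynamic grass system that caps how many times a fire can propagate.
; It keeps a running propagation count, raised through an increment function, and reports whether the maximum has been reached.
; On reaching the limit it schedules its own destruction after a long delay, so remaining instances that still want to propagate can query it.
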(event Custom|DestroyLater
  ;[1 1 1] It executes this after it's not needed anymore.
  (Utilities|FlowControl|Delay 2e+02)
  (Actor|DestroyActor))

(fn ConstructionScript)

(fn IncrementPropagationCounter
  ;[1 1 1] The most advanced function in Blueprint history.
  (Math|Integer|IncrementInt (Variables|Default|GetcurrentPropagations)))

(fn HasReachedMaxPropagations
  ;[1 1 1] It checks if current propagation amount has reached its maximum value.
  ; If so, destroy itself after a few minutes (to give some time for any remaining instances that can want to propagate)
  (if (>= (Variables|Default|GetcurrentPropagations) (Variables|Default|GetmaxPropagationAmount))
    (CallFunction|DestroyLater)
    (return true)
    (else
      (return false))))