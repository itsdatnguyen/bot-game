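; InteractiveFoliageChunk_BP is a foliage chunk in the dynamic grass system that links its foliage component to a Manager.
; Its construction script either keeps the default component, points FoliageComponent at SourceFoliageComp, or copies that source's foliage parameters into the existing component.
; Two flags, LeaveDefaultComponent and ReplaceWithSourceComponent, select the path, and every path assigns the Manager to the resulting component.
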(fn ConstructionScript
  (if (Variables|Default|GetleaveDefaultComponent)
    (Variables|/Game/DynamicGrassSystem/Blueprints/InternalLogic/INTERACTIVE_FoliageComp_BP.INTERACTIVE_FoliageComp_BP_C|SetManager (Variables|Default|GetFoliageComponent) (Variables|Default|Getmanager))
    (elif (Variables|Default|GetreplaceWithSourceComponent)
      (Variables|Default|SetFoliageComponent (Variables|Default|GetsourceFoliageComp))
      (Variables|/Game/DynamicGrassSystem/Blueprints/InternalLogic/INTERACTIVE_FoliageComp_BP.INTERACTIVE_FoliageComp_BP_C|SetManager (Variables|Default|GetFoliageComponent) (Variables|Default|Getmanager))
      (else
        (Variables|/Game/DynamicGrassSystem/Blueprints/InternalLogic/INTERACTIVE_FoliageComp_BP.INTERACTIVE_FoliageComp_BP_C|SetManager (Variables|Default|GetFoliageComponent) (Variables|Default|Getmanager))
        (Default|Copy&SetFoliageParameters (Variables|Default|GetFoliageComponent) (Variables|Default|GetsourceFoliageComp))))))